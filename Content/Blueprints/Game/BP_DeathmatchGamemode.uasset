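; Deathmatch game mode Blueprint that can end the round on a kill limit.
; It extends the parent's CharacterDead event, running the inherited handling first.
; When kill limiting is enabled, it reads the instigator's kill count from BP_PlayerState and calls StopRound with a KillLimit reason once that count reaches the limit.
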(event EventCharacterDead
  (params (DeadCharacter :type BP%20Player%20Character%20Object%20Reference) (DeathInstigator :type BP%20Player%20Controller%20Object%20Reference) (DeathCauseBy :type Actor%20Object%20Reference))
  (|CallParentFunction DeadCharacter DeathInstigator DeathCauseBy)
  (if (Variables|Limit|GetLimitByKills)
    (if (>= (Variables|/Game/Blueprints/Player/BP_PlayerState.BP_PlayerState_C|GetKills (.AsBP%20Player%20State (Utilities|Casting|CastToBP_PlayerState (Variables|/Script/Engine.Controller|GetPlayerState DeathInstigator)))) (Variables|Limit|GetKillsLimit))
      (CallFunction|StopRound "KillLimit"))))

(fn ConstructionScript
  (|CallParentFunction))