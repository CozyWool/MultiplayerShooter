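; Game state Blueprint that tracks points for two teams, TeamA and TeamB.
; BeginPlay sizes a point array to match the team points map.
; AddTeamPoints adds a value to both the map and the array, using a Select to turn the team into an array index.
; GetPoints reads a team's score from the array only.
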(event EventBeginPlay
  (|CallParentFunction)
  (Utilities|Array|Resize (Variables|Default|GetPointArray) (Utilities|Map|Length (Variables|Default|GetTeamPoints))))

(fn ConstructionScript
  (|CallParentFunction))

(fn AddTeamPoints
  (params (Team :type E_Team%20Enum%20%28by%20ref%29 :default "NewEnumerator0") (Value :type Integer))
  (bind _returnvalue (Utilities|Select :Index Team :NewEnumerator0 0 :NewEnumerator1 1))
  (Utilities|Map|Add (Variables|Default|GetTeamPoints) Team (+ (.Value (Utilities|Map|Find (Variables|Default|GetTeamPoints) Team)) Value))
  (Utilities|Array|SetArrayElem (Variables|Default|GetPointArray) _returnvalue (+ (Utilities|Array|Get(acopy) (Variables|Default|GetPointArray) _returnvalue) Value)))

(fn GetPoints
  (params (Team :type E_Team%20Enum :default "NewEnumerator0"))
  (return (Utilities|Array|Get(acopy) (Variables|Default|GetPointArray) (Utilities|Select :Index Team :NewEnumerator0 0 :NewEnumerator1 1))))