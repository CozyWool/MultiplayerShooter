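; Base GameState that tracks the round phase (pre-start, game, round end) and its timers for the match.
; A once-per-second server tick counts down to call the GameMode's StartRound, then advances round time and reports when the optional time limit is reached.
; The RoundInProgress RepNotify fires RoundStarted, while the GameMode's round-end event is multicast as RoundEnded with its reason.
; The GameMode round-start binding exists but is never run.
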(event EventBeginPlay
  (Networking|SwitchHasAuthority
    (:Authority
      (|BindRoundEnd))))

(event EventTick
  (params (DeltaSeconds :type Float%20%28single-precision%29))
  (Networking|SwitchHasAuthority
    (:Authority
      (switch Utilities|FlowControl|Switch|SwitchonE_GameState (Variables|Default|GetRoundInProgress)
        (:NewEnumerator0
          (bind _result (Math|Integer|DecrementInt (Variables|Default|GetRoundStartTime))
            (:%20%20
              (if (<= _result 0)
                (Default|StartRound (CallFunction|GetGamemode))
                (Variables|Default|SetRoundInProgress "NewEnumerator1")))))
        (:NewEnumerator1
          (CallFunction|RoundTimeTick))))))

(fn ConstructionScript)

(fn RoundTimeTick
  (bind _gamemode (CallFunction|GetGamemode))
  (bind _output_get (Variables|RoundTime|SetRoundTime (+ (Variables|RoundTime|GetRoundTime) (Math|Timespan|MakeTimespan 0 0 0 1))))
  (Variables|RoundTime|SetCurrentMinute (.Minutes (Math|Timespan|BreakTimespan _output_get)))
  (Variables|RoundTime|SetCurrentSecond (.Seconds (Math|Timespan|BreakTimespan _output_get)))
  (if (Math|Boolean|ANDBoolean (>= (Variables|RoundTime|GetRoundTime) (Variables|/Game/Blueprints/Game/BP_BaseGamemode.BP_BaseGamemode_C|GetTimeLimit _gamemode)) (Utilities|Enum|Equal(Enum) (Variables|Default|GetRoundInProgress) "NewEnumerator1") (Variables|/Game/Blueprints/Game/BP_BaseGamemode.BP_BaseGamemode_C|GetLimitByTime _gamemode)) ; Time limit reached
    (Default|TimeLimitReached (CallFunction|GetGamemode))
    (Variables|Default|SetRoundInProgress "NewEnumerator2")))

(fn GetRoundTime
  (return (Variables|RoundTime|GetCurrentMinute) (Variables|RoundTime|GetCurrentSecond)))

(fn OnRepRoundinProgress
  (switch Utilities|FlowControl|Switch|SwitchonE_GameState (Variables|Default|GetRoundInProgress)
    (:NewEnumerator1
      (Default|CallRoundStarted))))

(fn GetPreRoundTime
  (return (Variables|Default|GetRoundStartTime)))

(event Custom|OnRoundStarted
  (Variables|Default|SetRoundInProgress "NewEnumerator0"))

(event Custom|OnRoundEnded
  (params (Reason :type String))
  (CallFunction|Multicast-RoundEnd Reason)
  (Variables|Default|SetRoundInProgress "NewEnumerator2"))

(event Custom|Multicast-RoundEnd
  (params (Reason :type String))
  (Default|CallRoundEnded Reason))