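; BP_GameSpectator_CharFollow is a spectator Blueprint that smoothly follows an assigned character's location.
; SetFollowCharacter stores the target, and Tick interpolates the spectator toward it with VInterpTo while the target is valid, without sweeping.
; Movement runs only on the Remote (non-authority) side, which also changes the interpolation speed after a short delay following BeginPlay.
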(event EventBeginPlay
  (Networking|SwitchHasAuthority
    (:Remote
      (Utilities|FlowControl|Delay 1.0)
      (Variables|Default|SetInterp%20Speed 2e+01))))

(event EventTick
  (params (DeltaSeconds :type Float%20%28single-precision%29))
  (Networking|SwitchHasAuthority
    (:Remote
      (bind _followcharacter (Variables|Default|GetFollowCharacter)
        (:then
          (Transformation|SetActorLocation (Math|Interpolation|VInterpTo (Transformation|GetActorLocation) (Transformation|GetActorLocation _followcharacter) (Utilities|Time|GetWorldDeltaSeconds) (Variables|Default|GetInterp%20Speed)) false false))
        (:else)))))

(fn ConstructionScript
  (|CallParentFunction))

(fn SetFollowCharacter
  (params (FollowCharacter :type BP%20Player%20Character%20Object%20Reference))
  (Variables|Default|SetFollowCharacter FollowCharacter))