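; Base HUD that swaps the pre-round, in-game, spectate, tab and post-round widgets for the owning player.
; It binds to GameState round start and end events, then to the PlayerState alive and dead events once the round starts.
; Toggle functions lazily create each widget and reuse it, with some gated on game state or alive status.
; On death, the spectate widget receives instigator and causer info.
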(event Custom|OnRoundStarted
  (bind _returnvalue (Game|Player|GetOwningPlayerController))
  (bind _playerstate (CallFunction|GetPlayerStatebyController _returnvalue))
  ;[1 1 1] Round start and end
  (CallFunction|TogglePreRound false)
  (CallFunction|ToggleHUD true)
  (EventDispatchers|AssignPlayerAlive _playerstate (delegate Custom|OnPlayerAlive))
  (EventDispatchers|AssignPlayerDead _playerstate (delegate Custom|OnPlayerDead)))

(event Custom|OnPlayerAlive
  ;[1 1 1] When player revives
  (CallFunction|ToggleHUD true)
  (CallFunction|ToggleSpectate false))

(event Custom|OnPlayerDead
  (params (Instigator :type BP%20Player%20Character%20Object%20Reference) (DeathCauser :type Actor%20Object%20Reference) (Player :type BP%20Player%20State%20Object%20Reference))
  ;[1 1 1] When player dies
  (CallFunction|ToggleHUD false)
  (CallFunction|ToggleSpectate true)
  (if (CallFunction|IsGameinState "NewEnumerator1")
    (Default|SetDeathInfo (Variables|Default|GetSpectateWidget) Instigator DeathCauser)))

(event Custom|OnRoundEnded
  (params (Reason :type String))
  ;[1 1 1] Round start and end
  (CallFunction|ToggleHUD false)
  (CallFunction|ToggleSpectate false)
  (CallFunction|ToggleTab false)
  (CallFunction|TogglePostRound true))

(event EventBeginPlay
  (bind _out (CallFunction|GetGameState))
  ;[1 1 1] Round start and end
  (CallFunction|TogglePreRound true)
  (EventDispatchers|AssignRoundStarted _out (delegate Custom|OnRoundStarted))
  (EventDispatchers|AssignRoundEnded _out (delegate Custom|OnRoundEnded)))

(fn ConstructionScript)

(fn ToggleHUD
  (params (Show :type Boolean))
  (if Show
    (if (Variables|/Game/Blueprints/Player/BP_PlayerState.BP_PlayerState_C|GetAlive (CallFunction|GetPlayerStatebyController (Game|Player|GetOwningPlayerController)))
      (bind _hudwidget (Variables|Default|GetHUDWidget)
        (:then
          (UserInterface|Viewport|AddtoViewport _hudwidget 0))
        (:else
          (bind _returnvalue (UserInterface|CreateWidget (Variables|Default|GetHUDWidgetClass) (Game|Player|GetOwningPlayerController)))
          (bind _output_get (Variables|Default|SetHUDWidget _returnvalue))
          (UserInterface|Viewport|AddtoViewport _output_get 0))))
    (else
      (bind _hudwidget_2 (Variables|Default|GetHUDWidget)
        (:then
          (Widget|RemovefromParent _hudwidget_2))
        (:else)))))

(fn ToggleTab
  (params (Show :type Boolean))
  (if (CallFunction|IsGameinState "NewEnumerator1")
    (if Show
      (bind _tabwidget (Variables|Default|GetTabWidget)
        (:then
          (UserInterface|Viewport|AddtoViewport _tabwidget 0))
        (:else
          (bind _returnvalue (UserInterface|CreateWidget (Variables|Default|GetTabWidgetClass) (Game|Player|GetOwningPlayerController)))
          (bind _output_get (Variables|Default|SetTabWidget _returnvalue))
          (UserInterface|Viewport|AddtoViewport _output_get 0)))
      (else
        (bind _tabwidget_2 (Variables|Default|GetTabWidget)
          (:then
            (Widget|RemovefromParent _tabwidget_2))
          (:else))))))

(fn ToggleSpectate
  (params (Show :type Boolean))
  (if Show
    (if (CallFunction|IsGameinState "NewEnumerator1")
      (bind _spectatewidget (Variables|Default|GetSpectateWidget)
        (:then
          (UserInterface|Viewport|AddtoViewport _spectatewidget 0))
        (:else
          (bind _returnvalue (UserInterface|CreateWidget (Variables|Default|GetSpectateWidgetClass) (Game|Player|GetOwningPlayerController)))
          (bind _output_get (Variables|Default|SetSpectateWidget _returnvalue))
          (UserInterface|Viewport|AddtoViewport _output_get 0))))
    (else
      (bind _spectatewidget_2 (Variables|Default|GetSpectateWidget)
        (:then
          (Widget|RemovefromParent _spectatewidget_2))
        (:else)))))

(fn TogglePreRound
  (params (Show :type Boolean))
  (if Show
    (bind _preroundwidget (Variables|Default|GetPreRoundWidget)
      (:then
        (UserInterface|Viewport|AddtoViewport _preroundwidget 0))
      (:else
        (bind _returnvalue (UserInterface|CreateWidget (Variables|Default|GetPreRoundWidgetClass) (Game|Player|GetOwningPlayerController)))
        (bind _output_get (Variables|Default|SetPreRoundWidget _returnvalue))
        (UserInterface|Viewport|AddtoViewport _output_get 0)))
    (else
      (bind _preroundwidget_2 (Variables|Default|GetPreRoundWidget)
        (:then
          (Widget|RemovefromParent _preroundwidget_2))
        (:else)))))

(fn TogglePostRound
  (params (Show :type Boolean))
  (if Show
    (bind _postroundwidget (Variables|Default|GetPostRoundWidget)
      (:then
        (UserInterface|Viewport|AddtoViewport _postroundwidget 0))
      (:else
        (bind _returnvalue (UserInterface|CreateWidget (Variables|Default|GetPostRoundWidgetClass) (Game|Player|GetOwningPlayerController)))
        (bind _output_get (Variables|Default|SetPostRoundWidget _returnvalue))
        (UserInterface|Viewport|AddtoViewport _output_get 0)))
    (else
      (bind _postroundwidget_2 (Variables|Default|GetPostRoundWidget)
        (:then
          (Widget|RemovefromParent _postroundwidget_2))
        (:else)))))