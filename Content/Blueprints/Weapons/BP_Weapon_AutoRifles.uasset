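; BP_Weapon_AutoRifles is an auto rifle weapon Blueprint that displays its ammo count on a text render component.
; On BeginPlay it applies the WeaponSM mesh to the SIX12 static mesh component.
; Each Tick it calls the parent, then rewrites the text as current ammo over total ammo.
; The file contains no firing or reload logic, and its overlap event is disabled.
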(event Collision|EventActorBeginOverlap
  (params (OtherActor :type Actor%20Object%20Reference))
  (|CallParentFunction OtherActor) ; This node is disabled and will not be called.\nDrag off pins to build functionality.
)

(event EventTick
  (params (DeltaSeconds :type Float%20%28single-precision%29))
  (|CallParentFunction DeltaSeconds)
  (Rendering|Components|TextRender|SetText (Variables|Default|GetTextRender) (Utilities|Text|FormatText "{C} / {T}" (Variables|Default|GetCurrentAmmo) (Variables|Default|GetTotalAmmo))))

(event EventBeginPlay
  (Components|StaticMesh|SetStaticMesh (Variables|Default|GetSIX12) (Variables|Default|GetWeaponSM)))

(fn ConstructionScript
  (|CallParentFunction))