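; Firearm weapon Blueprint that extends a parent weapon with shooting, ammo and reloading.
; UseWeapon spawns FireProjectile if that class is set, otherwise applies point damage from a line trace, both starting at the player camera along the owner's forward vector.
; An empty magazine with reserve ammo sets Reloading, which blocks firing.
; Its OnRep runs the reload timer on authority, and ReloadFinished moves ammo from reserve to magazine.
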(event Custom|DEBUG_DrawServerTrace
  (params (Start :type Vector) (End :type Vector) (Hit :type Vector))
  (Rendering|Debug|DrawDebugLine Start End "(R=1.000000,G=0.815045,B=0.063137,A=1.000000)" 5.0 2.0)
  (Rendering|Debug|DrawDebugSphere Hit 4e+01 8 "(R=1.000000,G=0.000000,B=0.000000,A=1.000000)" 5.0 2.0))

(event EventBeginPlay
  (|CallParentFunction) ; This node is disabled and will not be called.\nDrag off pins to build functionality.
)

(event Collision|EventActorBeginOverlap
  (params (OtherActor :type Actor%20Object%20Reference))
  (|CallParentFunction OtherActor) ; This node is disabled and will not be called.\nDrag off pins to build functionality.
)

(event EventTick
  (params (DeltaSeconds :type Float%20%28single-precision%29))
  (|CallParentFunction DeltaSeconds) ; This node is disabled and will not be called.\nDrag off pins to build functionality.
)

(fn ConstructionScript
  (|CallParentFunction))

(fn UseWeapon
  (bind _used (|CallParentFunction))
  (if _used
    (if (Utilities|IsValidClass (Variables|Default|GetFireProjectile))
      (CallFunction|SpawnShootProjectile)
      (return true)
      (else
        (bind _hit (CallFunction|GetFireTrace))
        (Game|Damage|ApplyPointDamage (.HitActor (Collision|BreakHitResult _hit)) (Variables|Default|GetDamage) (Math|Vector|GetUnitDirection(Vector) (.TraceEnd (Collision|BreakHitResult _hit)) (.TraceStart (Collision|BreakHitResult _hit))) _hit (Game|GetInstigatorController) self)
        (return true)))
    (elif (and (<= (Variables|Default|GetCurrentAmmo) 0) (> (Variables|Default|GetTotalAmmo) 0))
      (Variables|Reload|SetReloading true)
      (return false)
      (else
        (return false)))))

(fn GetFireTrace
  (bind _asbp_player_character (Utilities|Casting|CastToBP_PlayerCharacter (Game|GetInstigator))
    (:then
      (bind _outhit (Collision|LineTraceForObjects (Transformation|GetWorldLocation (Variables|/Game/Blueprints/Player/BP_PlayerCharacter.BP_PlayerCharacter_C|GetCamera _asbp_player_character)) (+ (Transformation|GetWorldLocation (Variables|/Game/Blueprints/Player/BP_PlayerCharacter.BP_PlayerCharacter_C|GetCamera _asbp_player_character)) (* (Transformation|GetActorForwardVector (Components|GetOwner)) 10000)) (Utilities|Array|MakeArray "ObjectTypeQuery1" "ObjectTypeQuery2" "ObjectTypeQuery3") false (Utilities|Array|MakeArray self (Game|GetInstigator)) "None"))
      (CallFunction|DEBUGDrawServerTrace (.TraceStart (Collision|BreakHitResult _outhit)) (.TraceEnd (Collision|BreakHitResult _outhit)) (.Location (Collision|BreakHitResult _outhit)))
      (return _outhit))
    (:CastFailed
      (return ""))))

(fn ReloadFinished
  (Variables|Reload|SetReloading false)
  (Variables|Default|SetCurrentAmmo (+ (Variables|Reload|GetAmmoToReload) (Variables|Default|GetCurrentAmmo)))
  (Variables|Default|SetTotalAmmo (- (Variables|Default|GetTotalAmmo) (Variables|Reload|GetAmmoToReload))))

(fn OnRepReloading
  (Networking|SwitchHasAuthority
    (:Authority
      (if (Variables|Reload|GetReloading)
        (if (CallFunction|AbletoReload)
          (CallFunction|PrintMessage "Reloading" 2.0 "(R=1.000000,G=0.013877,B=0.980748,A=1.000000)" false)
          (bind _returnvalue (Utilities|Time|SetTimerbyFunctionName 0 "ReloadFinished" (Variables|Reload|GetReloadTime)))
          (Variables|Reload|SetReloadTImer _returnvalue)
          (Variables|Reload|SetAmmoToReload (Math|Integer|Min(Integer) (- (Utilities|GetClassDefaults (Utilities|GetClass self)) (Variables|Default|GetCurrentAmmo)) (Variables|Default|GetTotalAmmo)))
          (else
            (Variables|Reload|SetReloading false)
            (CallFunction|PrintMessage :Message "Not able to reload" :Duration 2.0 :Error true)))
        (else
          (Utilities|Time|ClearandInvalidateTimerbyHandle (Variables|Reload|GetReloadTImer)))))))

(fn AbletoReload
  (return (Math|Boolean|ANDBoolean (!= (.CurrentAmmo (Utilities|GetClassDefaults (Utilities|GetClass self))) (Variables|Default|GetCurrentAmmo)) (> (Variables|Default|GetTotalAmmo) 0) (not (Utilities|Time|IsValidTimerHandle (Variables|Reload|GetReloadTImer))))))

(fn AbletoUseWeapon
  (return (and (|CallParentFunction) (not (Variables|Reload|GetReloading)))))

(fn SpawnShootProjectile
  (bind _asbp_player_character (Utilities|Casting|CastToBP_PlayerCharacter (Game|GetInstigator)))
  (Game|SpawnActorfromClass (Variables|Default|GetFireProjectile) (Math|Transform|MakeTransform (+ (Transformation|GetWorldLocation (Variables|/Game/Blueprints/Player/BP_PlayerCharacter.BP_PlayerCharacter_C|GetCamera _asbp_player_character)) (* (Transformation|GetActorForwardVector (Components|GetOwner)) 70)) (Math|Conversions|RotationFromXVector (Transformation|GetActorForwardVector (Components|GetOwner)))) "AlwaysSpawn" self (Variables|Default|GetDamage) (Game|GetInstigator)))